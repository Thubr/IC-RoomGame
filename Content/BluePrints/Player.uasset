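; First-person style player Blueprint with mouse look, stepped arrow-key movement and hold-to-interact on whatever the camera faces.
; Tick line-traces from the camera and, while either mouse button is held, picks the action by actor display-name substring.
; Fans and certain doors rotate, books move against the view direction, and items are destroyed, counted and sent to the Inventory widget.
; Right click also prints the target's name, and releasing either button shows the Pointer.
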(event EventBeginPlay
  (Variables|Default|Setpaused true)
  (Rendering|SetVisibility (Variables|Default|GetPointer) false false)
  (Rendering|SetVisibility (Variables|Default|GetPointerMC) false false)
  (Variables|Default|SetshowTargetName false))

(event Collision|EventActorBeginOverlap
  (params (OtherActor :type Actor%20Object%20Reference)))

(event EventTick
  (params (DeltaSeconds :type Float%20%28single-precision%29))
  (bind _camera (Variables|Default|GetCamera))
  (bind _returnvalue (Transformation|GetWorldLocation _camera))
  (bind _outhit (Collision|LineTraceByChannel _returnvalue (+ _returnvalue (* (Math|Vector|GetForwardVector _camera) 1000)) "TraceTypeQuery2" false 0 "None"))
  (if (not (Variables|Default|Getpaused))
    (if (Variables|Default|GetshowTargetName)
      (Development|PrintString (Utilities|GetDisplayName (.HitActor (Collision|BreakHitResult _outhit))))
      (Variables|Default|SetshowTargetName false))
    (if (or (Utilities|String|Contains (Utilities|GetDisplayName (.HitActor (Collision|BreakHitResult _outhit))) "FanPivot") (Utilities|String|Contains (Utilities|GetDisplayName (.HitActor (Collision|BreakHitResult _outhit))) "door1_door3"))
      (Transformation|AddLocalRotation (Variables|/Script/Engine.Actor|GetRootComponent (.HitActor (Collision|BreakHitResult _outhit))) "0,1.000000, 0" false false)
      (elif (Utilities|String|Contains (Utilities|GetDisplayName (.HitActor (Collision|BreakHitResult _outhit))) "Book")
        (Transformation|AddActorLocalOffset "0, 0, 0" false false)
        (Transformation|AddWorldOffset (Variables|/Script/Engine.Actor|GetRootComponent (.HitActor (Collision|BreakHitResult _outhit))) (* (Math|Vector|GetForwardVector (Variables|Default|GetCamera)) -1.0) false false)
        (elif (Utilities|String|Contains (Utilities|GetDisplayName (.HitActor (Collision|BreakHitResult _outhit))) "Item")
          (Math|Integer|IncrementInt (Utilities|Array|Get(acopy) (Variables|Default|Getinv))
            (:%20%20
              (Actor|DestroyActor (.HitActor (Collision|BreakHitResult _outhit)))
              (bind _asinventory (Utilities|Casting|CastToInventory (UserInterface|GetUserWidgetObject (Variables|Default|GetWidget)))
                (:then
                  (Default|NewItem _asinventory))
                (:CastFailed
                  (Class|VisualLoggerKismetLibrary|LogText 0 "failed" "VisLogBP"))))))))))

(event Input|MouseEvents|MouseX
  (params (AxisValue :type Float%20%28single-precision%29))
  (Pawn|Input|AddControllerYawInput AxisValue))

(event Input|MouseEvents|MouseY
  (params (AxisValue :type Float%20%28single-precision%29))
  (Pawn|Input|AddControllerPitchInput (* -1 AxisValue)))

(event Input|KeyboardEvents|Right
  (params (Key :type Key%20Structure))
  (:Pressed
    (Transformation|AddActorWorldOffset (* (Math|Vector|ProjectVectorontoPlane (Math|Vector|GetRightVector (Variables|Default|GetCamera)) "0, 0, 0") 5e+01))))

(event Input|KeyboardEvents|Up
  (params (Key :type Key%20Structure))
  (:Pressed
    (Transformation|AddActorWorldOffset (* (Math|Vector|ProjectVectorontoPlane (Math|Vector|GetForwardVector (Variables|Default|GetCamera)) "0, 0,1.000000") 5e+01))))

(event Input|MouseEvents|RightMouseButton
  (params (Key :type Key%20Structure))
  (bind _pointer (Variables|Default|GetPointer))
  (:Pressed
    (Variables|Default|SetshowTargetName true)
    (Variables|Default|Setpaused false)
    (Rendering|SetVisibility _pointer false false))
  (:Released
    (Variables|Default|Setpaused true)
    (Rendering|SetVisibility _pointer true false)))

(event Input|KeyboardEvents|Down
  (params (Key :type Key%20Structure))
  (:Pressed
    (Transformation|AddActorWorldOffset (* (* (Math|Vector|ProjectVectorontoPlane (Math|Vector|GetForwardVector (Variables|Default|GetCamera)) "0, 0,1.000000") 5e+01) -1))))

(event Input|KeyboardEvents|Left
  (params (Key :type Key%20Structure))
  (:Pressed
    (Transformation|AddActorWorldOffset (* (* (Math|Vector|ProjectVectorontoPlane (Math|Vector|GetRightVector (Variables|Default|GetCamera)) "0, 0, 0") 5e+01) -1))))

(event Input|MouseEvents|LeftMouseButton
  (params (Key :type Key%20Structure))
  (bind _pointer (Variables|Default|GetPointer))
  (:Pressed
    (Variables|Default|SetshowTargetName false)
    (Variables|Default|Setpaused false)
    (Rendering|SetVisibility _pointer false false))
  (:Released
    (Variables|Default|Setpaused true)
    (Rendering|SetVisibility _pointer true false)))

(fn ConstructionScript)